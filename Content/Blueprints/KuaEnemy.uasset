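; Kua enemy that travels along a spline and shoots the player, Diana, on sight.
; A BeginPlay timeline moves the spinning capsule along the spline, with a health-bar plane floating above it.
; A per-tick forward line trace spotting Diana applies damage to her, throttled by a DoOnce and delay reset.
; Taking damage shrinks the bar and flashes the body red, and zero health plays death sounds and destroys the actor.
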(event EventBeginPlay
  (bind _spline (Variables|Default|GetSpline))
  (bind _capsule (Variables|Default|GetCapsule))
  (bind _returnvalue (Transformation|GetWorldRotation _capsule))
  (bind _newtrack (Timeline|Timeline_0 Play)
    (:Update
      (Transformation|SetWorldLocationAndRotation _capsule (Math|Vector|MakeVector (.x (Spline|GetLocationatDistanceAlongSpline _spline (Math|Float|Lerp 0.0 (Spline|GetSplineLength _spline) _newtrack) "World")) (.y (Spline|GetLocationatDistanceAlongSpline _spline (Math|Float|Lerp 0.0 (Spline|GetSplineLength _spline) _newtrack) "World")) (.z (Spline|GetLocationatDistanceAlongSpline _spline (Math|Float|Lerp 0.0 (Spline|GetSplineLength _spline) _newtrack) "World"))) (Math|Rotator|MakeRotator (+ (.roll (Transformation|GetWorldRotation _capsule)) 1.0) 0.0 (+ (.yaw (Spline|GetRotationatDistanceAlongSpline _spline (Math|Float|Lerp 0.0 (Spline|GetSplineLength _spline) _newtrack) "World")) -9e+01)) false false)
      (Transformation|SetWorldRotation _capsule (Math|Rotator|MakeRotator (+ (.roll _returnvalue) 1.0) (.pitch _returnvalue) (.yaw _returnvalue)) false false)
      (Transformation|SetWorldLocationAndRotation (Variables|Default|GetPlane2) (Math|Vector|MakeVector (.x (Spline|GetLocationatDistanceAlongSpline _spline (Math|Float|Lerp 0.0 (Spline|GetSplineLength _spline) _newtrack) "World")) (.y (Spline|GetLocationatDistanceAlongSpline _spline (Math|Float|Lerp 0.0 (Spline|GetSplineLength _spline) _newtrack) "World")) (+ (.z (Spline|GetLocationatDistanceAlongSpline _spline (Math|Float|Lerp 0.0 (Spline|GetSplineLength _spline) _newtrack) "World")) 75.0)) (Math|Rotator|MakeRotator 9e+01 9e+01 (.yaw _returnvalue)) false false))))

(event Collision|EventActorBeginOverlap
  (params (OtherActor :type Actor%20Object%20Reference)))

(event EventTick
  (params (DeltaSeconds :type Float%20%28single-precision%29))
  (bind _capsule (Variables|Default|GetCapsule))
  (bind _returnvalue (Transformation|GetWorldLocation _capsule))
  (bind _returnvalue_2 (Transformation|GetWorldRotation _capsule))
  (bind _outhit (Collision|LineTraceByChannel _returnvalue (+ _returnvalue (* (Math|Vector|GetForwardVector (Math|Rotator|MakeRotator (.roll _returnvalue_2) (.pitch _returnvalue_2) (+ (.yaw _returnvalue_2) 9e+01))) 1.5e+03)) "TraceTypeQuery2" false 0 "None" true "(R=0.000000,G=0.128749,B=1.000000,A=0.000000)" "(R=0.000000,G=1.000000,B=0.000000,A=0.000000)"))
  (Utilities|Casting|CastToDiana (.HitActor (Collision|BreakHitResult _outhit)))
  (Utilities|FlowControl|DoOnce false :!label _label
    (:Completed
      (Development|PrintString "Kua sees you!")
      (Audio|PlaySoundatLocation "/Game/Sounds/pistol.pistol" (Transformation|GetWorldLocation (Variables|Default|GetCapsule)) "0, 0, 0" 1.0 1.0 0.0 0 0 0)
      (bind _asdiana (Utilities|Casting|CastToDiana (Game|GetPlayerCharacter 0)))
      (Game|Damage|ApplyDamage _asdiana 1e+01 0 0)
      (Utilities|FlowControl|Delay 2.0)
      (goto _label Reset))))

(event Game|Damage|EventAnyDamage
  (params (Damage :type Float%20%28single-precision%29) (DamageType :type Damage%20Type%20Object%20Reference) (InstigatedBy :type Controller%20Object%20Reference) (DamageCauser :type Actor%20Object%20Reference))
  (bind _capsule (Variables|Default|GetCapsule))
  (bind _plane2 (Variables|Default|GetPlane2))
  (bind _returnvalue (Transformation|GetWorldLocation _capsule))
  (bind _relativescale3d (Variables|/Script/Engine.SceneComponent|GetRelativeScale3D _plane2))
  (bind _output_get (Variables|Default|SetHealth (- (Variables|Default|GetHealth) Damage)))
  (Transformation|SetRelativeScale3D (Variables|Default|GetPlane2) (Math|Vector|MakeVector (.x _relativescale3d) (Math|Float|Clamp(Float) (/ _output_get 1e+02)) (.z _relativescale3d)))
  (Audio|PlaySoundatLocation "/Game/Sounds/DamageKua.DamageKua" _returnvalue "0, 0, 0" 1.0 1.0 0.0 0 0 0)
  (Rendering|Material|SetMaterial (Variables|Default|GetSphere1) 0 "/Game/Female_Mannequin/Materials/Female_Mannequin/MI_FemaleMannequin_body_red.MI_FemaleMannequin_body_red")
  (Utilities|FlowControl|Delay 0.2)
  (Rendering|Material|SetMaterial (Variables|Default|GetSphere1) 0 "/Game/Female_Mannequin/Materials/Female_Mannequin/M_FemaleMannequin_joints.M_FemaleMannequin_joints")
  (if (<= _output_get 0.0)
    (Audio|PlaySoundatLocation "/Game/Sounds/KillKua.KillKua" _returnvalue "0, 0, 0" 1.0 1.0 0.0 0 0 0)
    (Utilities|FlowControl|Sequence
      (:then_0
        (bind _asdiana (Utilities|Casting|CastToDiana (Game|GetPlayerCharacter 0)))
        (Audio|PlaySoundatLocation "/Game/Sounds/bam_bam.bam_bam" (Transformation|GetWorldLocation (Variables|/Game/Blueprints/Diana.Diana_C|GetCamera _asdiana)) "0, 0, 0" 1.0 1.0 0.0 0 0 _asdiana))
      (:then_1
        (Actor|DestroyActor)))))

(fn ConstructionScript)