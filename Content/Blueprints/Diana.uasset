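; Diana is a first-person player character with movement, single jump, capsule-height crouch and four weapons: pistol, rifle, sniper and raygun.
; Mouse wheel sets GunIndex, which Tick uses to apply mesh, offsets and stats; aiming repositions gun and muzzle flash.
; Camera line traces damage characters and push cubes, repeating while held for the rifle.
; The raygun destroys a hit character or cube, then spawns its class at the next shot's impact.
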(event EventBeginPlay
  ;[1 1 1] UI
  (Audio|Components|Audio|Stop (Variables|Default|GetGunLoop)))

(event EventTick
  (params (DeltaSeconds :type Float%20%28single-precision%29))
  (bind _gun (Variables|Default|GetGun))
  (Utilities|FlowControl|Sequence
    (:then_0
      (switch int (Variables|Default|GetGunIndex)
        (:Default
          (Components|StaticMesh|SetStaticMesh _gun "/Game/Guns/Pistol.Pistol"))
        (:0
          (if (Variables|Default|GetindexChange)
            (|PistolLocation _gun)))
        (:1
          (if (Variables|Default|GetindexChange)
            (|RifleLocation _gun)))
        (:2
          (if (Variables|Default|GetindexChange)
            (Components|StaticMesh|SetStaticMesh _gun "/Game/Guns/Sniper_rifle.Sniper_rifle")
            (|SniperLocation)))
        (:3
          (Components|StaticMesh|SetStaticMesh _gun "/Game/Guns/Ray_Gun.Ray_Gun")
          (|RaygunLocation))))
    (:then_1
      (if (Variables|Default|GetEnemySeesYou)
        _))))

(event EventOnLanded
  (params (Hit :type Hit%20Result%20Structure%20%28by%20ref%29))
  ;[1 1 1] Jumping
  (Utilities|FlowControl|DoOnce false) ; enters at Reset
)

(event Input|ActionEvents|InputActionAimDownSight
  (params (Key :type Key%20Structure :default "None"))
  ;[1 1 1] Aim Down Sight
  (:Pressed
    (switch int (Variables|Default|GetGunIndex)
      (:Default
        (bind (_gun _muzzleflash) (|PistolADS :!label _label)))
      (:0
        (Viewport|RemoveAllWidgets)
        (goto _label))
      (:1
        (|RifleADS))
      (:2
        (Viewport|RemoveAllWidgets)
        (|SniperADS))
      (:3
        (Viewport|RemoveAllWidgets)
        (|RaygunADS))))
  (:Released
    (bind _returnvalue (UserInterface|CreateWidget "/Game/UI/Reticle.Reticle_C" (Game|GetPlayerController 0)))
    (UserInterface|Viewport|AddtoViewport _returnvalue 0)
    (switch int (Variables|Default|GetGunIndex)
      (:Default
        (|PistolHip _gun _muzzleflash :!label _label_2))
      (:0
        (goto _label_2))
      (:1
        (|RifleHip))
      (:2
        (|SniperHip))
      (:3
        (|PistolHip_2 _gun _muzzleflash)))))

(event Input|AxisEvents|InputAxisMoveForward
  (params (AxisValue :type Float%20%28single-precision%29))
  ;[1 1 1] Movement
  (Pawn|Input|AddMovementInput (Math|Vector|GetForwardVector (Variables|Default|GetCamera)) AxisValue false))

(event Input|AxisEvents|InputAxisMoveRight
  (params (AxisValue :type Float%20%28single-precision%29))
  ;[1 1 1] Movement
  (Pawn|Input|AddMovementInput (Math|Vector|GetRightVector (Variables|Default|GetCamera)) AxisValue false))

(event Input|AxisEvents|InputAxisMouseVertical
  (params (AxisValue :type Float%20%28single-precision%29))
  ;[1 1 1] Camera
  (Pawn|Input|AddControllerPitchInput AxisValue))

(event Input|AxisEvents|InputAxisMouseHorizontal
  (params (AxisValue :type Float%20%28single-precision%29))
  ;[1 1 1] Camera
  (Pawn|Input|AddControllerYawInput AxisValue))

(event Input|MouseEvents|MouseWheelAxis
  (params (AxisValue :type Float%20%28single-precision%29))
  ;[1 1 1] Weapon Changing
  (if (not (== AxisValue 0.0))
    (if (not (or (< (Variables|Default|GetGunIndex) 0) (> (Variables|Default|GetGunIndex) 4)))
      (bind _output_get (Variables|Default|SetGunIndex (Math|Integer|Clamp(Integer) (Math|Float|Truncate (+ AxisValue (Math|Conversions|ToFloat(Integer) (Variables|Default|GetGunIndex)))) 0 3)))
      (Variables|Default|SetindexChange true)
      (Development|PrintString (Utilities|String|ToString(Integer) _output_get)))))

(event Input|MouseEvents|LeftMouseButton
  (params (Key :type Key%20Structure :default "None"))
  (bind _weaponrange (Variables|Default|GetWeaponRange))
  (bind _camera (Variables|Default|GetCamera))
  (bind _weaponrange_2 (Variables|Default|GetWeaponRange))
  (bind _camera_2 (Variables|Default|GetCamera))
  (bind _returnvalue (Transformation|GetWorldLocation _camera_2))
  (bind _returnvalue_2 (Math|Vector|GetForwardVector _camera_2))
  (bind _returnvalue_3 (Transformation|GetWorldLocation _camera))
  (bind _returnvalue_4 (Math|Vector|GetForwardVector _camera))
  (bind _returnvalue_5 (* _returnvalue_4 _weaponrange))
  (bind _returnvalue_6 (* _returnvalue_2 _weaponrange_2))
  (bind _returnvalue_7 (+ _returnvalue _returnvalue_6))
  (bind _returnvalue_8 (+ _returnvalue_3 _returnvalue_5))
  (:Pressed
    (Variables|Default|SetmousePressed true)
    (Utilities|FlowControl|Sequence
      (:then_0
        ;[1 1 1] Raygun Code
        (if (== (Variables|Default|GetGunIndex) 3)
          (if (Variables|Default|GetGunFilled)
            (bind _outhit (Collision|LineTraceByChannel _returnvalue _returnvalue_7 "TraceTypeQuery1" false 0 "None"))
            (Game|SpawnActorfromClass (Utilities|GetClass (Variables|Default|GetStoredObject)) (Math|Transform|MakeTransform (.Location (Collision|BreakHitResult _outhit)) "0, 0, 0" "1,1,1") "Undefined" 0 0)
            (Variables|Default|SetGunFilled false)
            (else
              (bind _outhit_2 (Collision|LineTraceByChannel _returnvalue _returnvalue_7 "TraceTypeQuery1" false 0 "Persistent"))
              (bind _asue_4asp_character (Utilities|Casting|CastToUe4ASP_Character (.HitActor (Collision|BreakHitResult _outhit_2)))
                (:then
                  (bind _output_get (Variables|Default|SetStoredObject _asue_4asp_character)))
                (:CastFailed
                  (bind _ascube (Utilities|Casting|CastToCube (.HitActor (Collision|BreakHitResult _outhit_2))))
                  (bind _output_get_2 (Variables|Default|SetStoredObject _ascube))))
              (Actor|DestroyActor _output_get)
              (Variables|Default|SetGunFilled true)))
          (else
            ;[1 1 1] Shoot Detection
            (bind _outhit_3 (Collision|LineTraceByChannel _returnvalue_3 _returnvalue_8 "TraceTypeQuery1" false 0 "None" :!label _label))
            (Utilities|FlowControl|Sequence
              (:then_0
                (bind _asue_4asp_character_2 (Utilities|Casting|CastToUe4ASP_Character (.HitActor (Collision|BreakHitResult _outhit_3))))
                (Development|PrintString "hit enemy")
                (Game|Damage|ApplyDamage _asue_4asp_character_2 (Variables|Default|GetWeaponDamage) 0 0))
              (:then_1
                (bind _ascube_2 (Utilities|Casting|CastToCube (.HitActor (Collision|BreakHitResult _outhit_3))))
                (Physics|SetPhysicsLinearVelocity (Variables|/Game/Blueprints/Cube.Cube_C|GetCube _ascube_2) (* (Math|Vector|Normalize (- _returnvalue_8 _returnvalue_3)) (Variables|Default|GetPunch-Through)) true "None"))
              (:then_2
                (if (== (Variables|Default|GetGunIndex) 1)
                  (if (Variables|Default|GetmousePressed)
                    (Utilities|FlowControl|Delay (Variables|Default|GetRifleRate))
                    (goto _label))))))))
      (:then_1
        ;[1 1 1] effects and audio
        (Utilities|FlowControl|DoOnce false :!label _label_2
          (:Completed
            (Utilities|FlowControl|Sequence
              (:then_0
                (switch int (Variables|Default|GetGunIndex)
                  (:0
                    (|PistolSFX))
                  (:1
                    (|RifleSFX))
                  (:2
                    (|SniperSFX))
                  (:3
                    (|RaygunSFX))))
              (:then_1
                (switch int (Variables|Default|GetGunIndex)
                  (:0
                    (|Pistolfire))
                  (:1
                    (|RifleFire))
                  (:2
                    (|SniperFire))))))))))
  (:Released
    (Variables|Default|SetmousePressed false)
    (Rendering|SetVisibility (Variables|Default|GetMuzzleFlash) false false)
    (Audio|Components|Audio|Stop (Variables|Default|GetGunLoop))
    (goto _label_2 Reset)))

(event Input|KeyboardEvents|SpaceBar
  (params (Key :type Key%20Structure :default "None"))
  ;[1 1 1] Jumping
  (:Pressed
    (Utilities|FlowControl|DoOnce false
      (:Completed
        (Character|LaunchCharacter "0, 0,400.000000" false false)))))

(event Input|KeyboardEvents|LeftCtrl
  (params (Key :type Key%20Structure :default "None"))
  (bind _capsulecomponent (Variables|Collision|GetCapsuleComponent))
  ;[1 1 1] Crouching
  (:Pressed
    (Components|Capsule|SetCapsuleHalfHeight _capsulecomponent 44.0 true))
  (:Released
    (Components|Capsule|SetCapsuleHalfHeight _capsulecomponent 88.0 true)))

(fn ConstructionScript)