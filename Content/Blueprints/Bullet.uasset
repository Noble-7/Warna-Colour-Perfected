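; Bullet is a physics-driven projectile actor that launches in the direction the player is looking.
; On BeginPlay it casts the player character to Diana and applies a large force to its Sphere along the forward vector of Diana's camera.
; It prints that force vector and the name of any overlapping actor, with no damage or destroy logic.
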(event EventBeginPlay
  (bind _asdiana (Utilities|Casting|CastToDiana (Game|GetPlayerCharacter 0)))
  (Physics|AddForce (Variables|Default|GetSphere) (* (Math|Vector|GetForwardVector (Variables|/Game/Blueprints/Diana.Diana_C|GetCamera _asdiana)) 1e+04) "None" false)
  (Development|PrintString (Utilities|String|ToString(Vector) (* (Math|Vector|GetForwardVector (Variables|/Game/Blueprints/Diana.Diana_C|GetCamera _asdiana)) 1e+04))))

(event Collision|EventActorBeginOverlap
  (params (OtherActor :type Actor%20Object%20Reference))
  (Development|PrintString (Utilities|GetDisplayName OtherActor)))

(event EventTick
  (params (DeltaSeconds :type Float%20%28single-precision%29)))

(fn ConstructionScript)