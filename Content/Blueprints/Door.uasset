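; Door Blueprint that swings open only while two linked buttons are both active.
; Each Tick casts its two button references to Button and checks their IsActive flags.
; When both are active it snaps to a 90-degree relative yaw and sets IsOpen; otherwise it resets to zero rotation and clears the flag.
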(event EventBeginPlay)

(event Collision|EventActorBeginOverlap
  (params (OtherActor :type Actor%20Object%20Reference)))

(event EventTick
  (params (DeltaSeconds :type Float%20%28single-precision%29))
  (bind _asbutton (Utilities|Casting|CastToButton (Variables|Default|Getbutton1Reference)))
  (bind _asbutton_2 (Utilities|Casting|CastToButton (Variables|Default|Getbutton2Reference)))
  (if (and (Variables|/Game/Blueprints/Button.Button_C|GetisActive _asbutton) (Variables|/Game/Blueprints/Button.Button_C|GetisActive _asbutton_2))
    (Transformation|SetActorRelativeRotation "0,90.000000, 0")
    (Variables|Default|SetisOpen true)
    (else
      (Transformation|SetActorRelativeRotation "0, 0, 0")
      (Variables|Default|SetisOpen false))))

(fn ConstructionScript)